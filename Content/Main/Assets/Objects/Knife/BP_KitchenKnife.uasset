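; Kitchen knife with a grab component that slices broccoli, bread, tomato, mushroom and sausage objects it hits.
; On a hit against a procedural mesh, a cast chain finds the food type and calls its Slice at the impact point, using the knife's up vector as plane normal.
; A slice starts a short cooldown that ignores PhysicsBody collision, then sets all channels to Block.
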(event OnComponentHit(SM_KitchenKnife)
  (params (HitComponent :type Primitive%20Component%20Object%20Reference) (OtherActor :type Actor%20Object%20Reference) (OtherComp :type Primitive%20Component%20Object%20Reference) (NormalImpulse :type Vector :default "0, 0, 0") (Hit :type Hit%20Result%20Structure%20%28by%20ref%29))
  (bind _impactpoint (Collision|BreakHitResult Hit))
  (bind _sm_kitchenknife (Variables|Default|GetSM_KitchenKnife))
  (bind _sm_kitchenknife_2 (Variables|Default|GetSM_KitchenKnife))
  (bind _returnvalue (Math|Vector|GetUpVector _sm_kitchenknife))
  (if (not (Variables|Default|GetCut%20Cooldown))
    (bind _asprocedural_mesh_component (Utilities|Casting|CastToProceduralMeshComponent OtherComp))
    ;[1 1 1] I am aware this is horrible, i just dont care
    (bind _asbp_broccoli (Utilities|Casting|CastToBP_Broccoli (Components|GetOwner _asprocedural_mesh_component))
      (:then
        (Default|Slice _asbp_broccoli _impactpoint _returnvalue _asprocedural_mesh_component))
      (:CastFailed
        (bind _asbp_bread (Utilities|Casting|CastToBP_Bread (Components|GetOwner _asprocedural_mesh_component))
          (:then
            (Default|Slice _asbp_bread _impactpoint _returnvalue _asprocedural_mesh_component))
          (:CastFailed
            (bind _asbp_tomato (Utilities|Casting|CastToBP_Tomato (Components|GetOwner _asprocedural_mesh_component))
              (:then
                (Default|Slice _asbp_tomato _impactpoint _returnvalue _asprocedural_mesh_component))
              (:CastFailed
                (bind _asbp_mushroom (Utilities|Casting|CastToBP_Mushroom (Components|GetOwner _asprocedural_mesh_component))
                  (:then
                    (Default|Slice _asbp_mushroom _impactpoint _returnvalue _asprocedural_mesh_component))
                  (:CastFailed
                    (bind _asbp_sausage (Utilities|Casting|CastToBP_Sausage (Components|GetOwner _asprocedural_mesh_component)))
                    (Default|Slice _asbp_sausage _impactpoint _returnvalue _asprocedural_mesh_component)))))))))
    (Variables|Default|SetCut%20Cooldown true)
    (Collision|SetCollisionResponsetoChannel _sm_kitchenknife_2 "ECC_PhysicsBody" "ECR_Ignore")
    (Utilities|FlowControl|Delay 1.0)
    (Variables|Default|SetCut%20Cooldown false)
    (Collision|SetCollisionResponsetoAllChannels _sm_kitchenknife_2 "ECR_Block")))

(event EventBeginPlay)

(event Collision|EventActorBeginOverlap
  (params (OtherActor :type Actor%20Object%20Reference)))

(event EventTick
  (params (DeltaSeconds :type Float%20%28single-precision%29)))

(fn ConstructionScript
  (Variables|/Game/VRTemplate/Blueprints/GrabComponent.GrabComponent_C|SetMeshReference (Variables|Default|GetGrabComponent) (Variables|Default|GetSM_KitchenKnife)))