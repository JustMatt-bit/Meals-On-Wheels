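; Grabbable broccoli object that can be sliced into separate physics pieces.
; The construction script copies the static mesh into a procedural mesh, adds convex collision from its vertices, destroys the original component and points the GrabComponent at the result.
; Slice cuts a given procedural mesh along a plane with a dark green cap, then enables physics and collision on the new half and attaches a new grab component to it.
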(event EventBeginPlay)

(event Collision|EventActorBeginOverlap
  (params (OtherActor :type Actor%20Object%20Reference)))

(event EventTick
  (params (DeltaSeconds :type Float%20%28single-precision%29)))

(fn ConstructionScript
  (bind _proceduralmesh (Variables|Default|GetProceduralMesh))
  (Utilities|FlowControl|Sequence
    (:then_0
      (Class|KismetProceduralMeshLibrary|CopyProceduralMeshfromStaticMeshComponent (Variables|Default|GetSM_Broccoli) 0 _proceduralmesh true)
      (bind _vertices (Class|KismetProceduralMeshLibrary|GetSectionfromStaticMesh "/Game/Main/Assets/Objects/Broccoli/SM_Broccoli.SM_Broccoli"))
      (Class|ProceduralMeshComponent|AddCollisionConvexMesh (Variables|Default|GetProceduralMesh) _vertices)
      (Components|DestroyComponent (Variables|Default|GetSM_Broccoli)))
    (:then_1
      (Variables|/Game/VRTemplate/Blueprints/GrabComponent.GrabComponent_C|SetMeshReference (Variables|Default|GetGrabComponent) _proceduralmesh))))

(fn Slice
  (params (Location :type Vector) (Slice%20Normal :type Vector) (Component%20To%20Slice :type Procedural%20Mesh%20Component%20Object%20Reference))
  (bind _outotherhalfprocmesh (Class|KismetProceduralMeshLibrary|SliceProceduralMesh Component%20To%20Slice Location Slice%20Normal true "CreateNewSectionForCap" "/Game/Main/Assets/Objects/Broccoli/Materials/M_BroccoliDarkGreen.M_BroccoliDarkGreen"))
  (Variables|Default|SetOtherHalf _outotherhalfprocmesh)
  (Physics|SetSimulatePhysics (Variables|Default|GetOtherHalf) true)
  (Collision|SetCollisionEnabled (Variables|Default|GetOtherHalf) "QueryAndPhysics")
  (bind _returnvalue (AddComponent|AddGrabComponent false))
  (Transformation|AttachComponentToComponent _returnvalue (Variables|Default|GetOtherHalf) "None" "KeepRelative" "KeepRelative" "KeepRelative" true))