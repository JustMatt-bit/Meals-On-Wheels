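; BP_Tomato is a tomato object that can be sliced into separate physics pieces that carry grab components.
; Its construction script copies the static mesh into a procedural mesh, adds convex collision and destroys the original component.
; Slice cuts the passed component along a given plane and caps it with red tomato material.
; The new half gets physics, collision and its own grab component, while the event graph stays empty.
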(event EventBeginPlay)

(event Collision|EventActorBeginOverlap
  (params (OtherActor :type Actor%20Object%20Reference)))

(event EventTick
  (params (DeltaSeconds :type Float%20%28single-precision%29)))

(fn ConstructionScript
  (Class|KismetProceduralMeshLibrary|CopyProceduralMeshfromStaticMeshComponent (Variables|Default|GetSM_Tomato) 0 (Variables|Default|GetProceduralMesh) true)
  (bind _vertices (Class|KismetProceduralMeshLibrary|GetSectionfromStaticMesh "/Game/Main/Assets/Objects/Tomato/SM_Tomato.SM_Tomato"))
  (Class|ProceduralMeshComponent|AddCollisionConvexMesh (Variables|Default|GetProceduralMesh) _vertices)
  (Components|DestroyComponent (Variables|Default|GetSM_Tomato)))

(fn Slice
  (params (Location :type Vector) (Slice%20Normal :type Vector) (Component%20To%20Slice :type Procedural%20Mesh%20Component%20Object%20Reference))
  (bind _outotherhalfprocmesh (Class|KismetProceduralMeshLibrary|SliceProceduralMesh Component%20To%20Slice Location Slice%20Normal true "CreateNewSectionForCap" "/Game/Main/Assets/Objects/Tomato/Materials/M_Tomato_Red.M_Tomato_Red"))
  (Variables|Default|SetOtherHalf _outotherhalfprocmesh)
  (Physics|SetSimulatePhysics (Variables|Default|GetOtherHalf) true)
  (Collision|SetCollisionEnabled (Variables|Default|GetOtherHalf) "QueryAndPhysics")
  (bind _returnvalue (AddComponent|AddGrabComponent false))
  (Transformation|AttachComponentToComponent _returnvalue (Variables|Default|GetOtherHalf) "None" "KeepRelative" "KeepRelative" "KeepRelative" true))