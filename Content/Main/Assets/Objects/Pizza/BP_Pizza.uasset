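; Grabbable pizza that gets topped with tomato, salami and mushroom actors and can then be cooked.
; Sphere overlaps tally overlapping actors of the incoming class; past each topping's threshold, it reveals that topping's component and destroys those actors.
; StartCooking swaps base and middle materials only once all three toppings are added.
; SpawnCooked makes the construction script show the finished pizza through SetAsCooked.
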(event OnComponentBeginOverlap(SphereOverlap)
  (params (OverlappedComponent :type Primitive%20Component%20Object%20Reference) (OtherActor :type Actor%20Object%20Reference) (OtherComp :type Primitive%20Component%20Object%20Reference) (OtherBodyIndex :type Integer) (bFromSweep :type Boolean) (SweepResult :type Hit%20Result%20Structure%20%28by%20ref%29))
  (bind _returnvalue (Utilities|GetClass OtherActor))
  (bind _overlappingactors (Collision|GetOverlappingActors OverlappedComponent _returnvalue :!class /Script/Engine.PrimitiveComponent))
  (for _array_element _overlappingactors
    (Utilities|Casting|CastToBP_Tomato _array_element
      (:then
        (if (not (Variables|Default|GetIs%20Tomato%20Added))
          (bind _result (Math|Integer|IncrementInt (Variables|Default|GetTomatoCount))
            (:%20%20
              (bind _output_get (Variables|Default|SetTomatoCount _result))
              (if (>= _output_get 6)
                (Rendering|SetVisibility (Variables|Default|GetTomatoes) true false)
                (for _array_element_2 _overlappingactors
                  (Actor|DestroyActor _array_element_2)
                  (Variables|Default|SetIs%20Tomato%20Added true)))))))
      (:CastFailed
        (Utilities|Casting|CastToBP_Sausage _array_element
          (:then
            (if (not (Variables|Default|GetIs%20Salami%20Added))
              (bind _result_2 (Math|Integer|IncrementInt (Variables|Default|GetSalamiCount))
                (:%20%20
                  (bind _output_get_2 (Variables|Default|SetSalamiCount _result_2))
                  (if (>= _output_get_2 10)
                    (Rendering|SetVisibility (Variables|Default|GetSalami) true false)
                    (for _array_element_3 _overlappingactors
                      (Actor|DestroyActor _array_element_3)
                      (Variables|Default|SetIs%20Salami%20Added true)))))))
          (:CastFailed
            (Utilities|Casting|CastToBP_Mushroom _array_element)
            (if (not (Variables|Default|GetIs%20Mushroom%20Added))
              (bind _result_3 (Math|Integer|IncrementInt (Variables|Default|GetMushroomCount))
                (:%20%20
                  (bind _output_get_3 (Variables|Default|SetMushroomCount _result_3))
                  (if (>= _output_get_3 7)
                    (Rendering|SetVisibility (Variables|Default|GetMushrooms) true false)
                    (for _array_element_4 _overlappingactors
                      (Actor|DestroyActor _array_element_4)
                      (Variables|Default|SetIs%20Mushroom%20Added true))))))))))))

(event Custom|StartCooking
  (if (not (Variables|Default|GetIs%20Cooked))
    (if (Variables|Default|GetIs%20Tomato%20Added)
      (if (Variables|Default|GetIs%20Mushroom%20Added)
        (if (Variables|Default|GetIs%20Salami%20Added)
          (Rendering|Material|SetMaterial (Variables|Default|GetPizzaBase) 0 "/Game/Main/Assets/Objects/Bread/Materials/M_Bread_DarkBrown.M_Bread_DarkBrown")
          (Rendering|Material|SetMaterial (Variables|Default|GetPizzaMiddle) 0 "/Game/Main/Assets/Objects/Pizza/Materials/Yellow.Yellow")
          (Variables|Default|SetIs%20Cooked true))))))

(fn ConstructionScript
  (Variables|/Game/VRTemplate/Blueprints/GrabComponent.GrabComponent_C|SetMeshReference (Variables|Default|GetGrabComponent) (Variables|Default|GetPizzaBase))
  (if (Variables|Default|GetSpawnCooked)
    (CallFunction|SetasCooked)))

(fn SetasCooked
  (Rendering|Material|SetMaterial (Variables|Default|GetPizzaBase) 0 "/Game/Main/Assets/Objects/Bread/Materials/M_Bread_DarkBrown.M_Bread_DarkBrown")
  (Rendering|Material|SetMaterial (Variables|Default|GetPizzaMiddle) 0 "/Game/Main/Assets/Objects/Pizza/Materials/Yellow.Yellow")
  (Variables|Default|SetIs%20Cooked true)
  (Rendering|SetVisibility (Variables|Default|GetTomatoes) true false)
  (Rendering|SetVisibility (Variables|Default|GetMushrooms) true false)
  (Rendering|SetVisibility (Variables|Default|GetSalami) true false))