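; BP_Bread is a grabbable bread object that can be sliced into separate physics pieces.
; Construction copies the static bread mesh into a procedural mesh with convex collision and an outline overlay, removes the original, and points the GrabComponent at the copy.
; Slice cuts a given procedural mesh along a plane with a light-brown cap, then enables physics and attaches a new GrabComponent to the severed half.
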(event EventBeginPlay)

(event Collision|EventActorBeginOverlap
  (params (OtherActor :type Actor%20Object%20Reference)))

(event EventTick
  (params (DeltaSeconds :type Float%20%28single-precision%29)))

(fn ConstructionScript
  (bind _proceduralmesh (Variables|Default|GetProceduralMesh))
  (bind _proceduralmesh_2 (Variables|Default|GetProceduralMesh))
  (Utilities|FlowControl|Sequence
    (:then_0
      (Class|KismetProceduralMeshLibrary|CopyProceduralMeshfromStaticMeshComponent (Variables|Default|GetSM_Bread) 0 _proceduralmesh true)
      (bind _vertices (Class|KismetProceduralMeshLibrary|GetSectionfromStaticMesh "/Game/Main/Assets/Objects/Bread/SM_Bread.SM_Bread"))
      (Class|ProceduralMeshComponent|AddCollisionConvexMesh _proceduralmesh_2 _vertices)
      (Components|DestroyComponent (Variables|Default|GetSM_Bread))
      (Rendering|Material|SetOverlayMaterial _proceduralmesh_2 "/Game/VRTemplate/Blueprints/M_Object_Outline.M_Object_Outline" :!class /Script/Engine.MeshComponent))
    (:then_1
      (Variables|/Game/VRTemplate/Blueprints/GrabComponent.GrabComponent_C|SetMeshReference (Variables|Default|GetGrabComponent) _proceduralmesh))))

(fn Slice
  (params (Location :type Vector) (Slice%20Normal :type Vector) (Component%20To%20Slice :type Procedural%20Mesh%20Component%20Object%20Reference))
  (bind _outotherhalfprocmesh (Class|KismetProceduralMeshLibrary|SliceProceduralMesh Component%20To%20Slice Location Slice%20Normal true "CreateNewSectionForCap" "/Game/Main/Assets/Objects/Bread/Materials/M_Bread_LightBrown.M_Bread_LightBrown"))
  (Variables|Default|SetOtherHalf _outotherhalfprocmesh)
  (Physics|SetSimulatePhysics (Variables|Default|GetOtherHalf) true)
  (Collision|SetCollisionEnabled (Variables|Default|GetOtherHalf) "QueryAndPhysics")
  (bind _returnvalue (AddComponent|AddGrabComponent false))
  (Transformation|AttachComponentToComponent _returnvalue (Variables|Default|GetOtherHalf) "None" "KeepRelative" "KeepRelative" "KeepRelative" true))