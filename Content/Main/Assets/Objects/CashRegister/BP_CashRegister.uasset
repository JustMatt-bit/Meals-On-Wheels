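; Cash register actor that banks the money left inside it into the player's saved balance on the game instance.
; A physics constraint reference is set at start, and an overlap on the back collision zone signals closing.
; Closing destroys each BP_Money in the detection zone and adds its value to a never-reset total.
; That running total is added to the game instance's Money once per item.
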(event OnComponentBeginOverlap(BackCollisionZone)
  (params (OverlappedComponent :type Primitive%20Component%20Object%20Reference) (OtherActor :type Actor%20Object%20Reference) (OtherComp :type Primitive%20Component%20Object%20Reference) (OtherBodyIndex :type Integer) (bFromSweep :type Boolean) (SweepResult :type Hit%20Result%20Structure%20%28by%20ref%29))
  ;[1 1 1] When cash register is closed, add all up all money inside
  (bind _output_get (Variables|Default|SetCashInRegister (Collision|GetOverlappingActors (Variables|Default|GetMoneyDetectionZone) "/Game/Main/Assets/Objects/CashRegister/Money/BP_Money.BP_Money_C" :!class /Script/Engine.PrimitiveComponent)))
  (for _array_element _output_get
    (bind _asbp_money (Utilities|Casting|CastToBP_Money _array_element))
    (bind _output_get_2 (Variables|Default|SetTotalInRegister (+ (Variables|Default|GetTotalInRegister) (Variables|/Game/Main/Assets/Objects/CashRegister/Money/BP_Money.BP_Money_C|GetValue _asbp_money))))
    (Actor|DestroyActor _asbp_money)
    (bind _asbp_main_game_instance (Utilities|Casting|CastToBP_MainGameInstance (Game|GetGameInstance)))
    (Variables|/Game/Main/Levels/BP_MainGameInstance.BP_MainGameInstance_C|SetMoney _asbp_main_game_instance (+ _output_get_2 (Variables|/Game/Main/Levels/BP_MainGameInstance.BP_MainGameInstance_C|GetMoney _asbp_main_game_instance)))))

(event EventBeginPlay
  (Class|PhysicsConstraintComponent|SetConstraintReferencePosition (Variables|Default|GetPhysicsConstraint) "Frame1" (Math|Vector|MakeVector 0.0 0.0 0.0))
  (Variables|Default|SetTotalInRegister 0.0))

(event Collision|EventActorBeginOverlap
  (params (OtherActor :type Actor%20Object%20Reference)))

(event EventTick
  (params (DeltaSeconds :type Float%20%28single-precision%29)))

(fn ConstructionScript)