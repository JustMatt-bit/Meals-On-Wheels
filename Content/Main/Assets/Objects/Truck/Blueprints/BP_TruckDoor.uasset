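; Truck door actor that slides its static mesh vertically, but only in the L_Menu_Map level.
; On BeginPlay it raises the mesh with an eased MoveComponentTo and plays the door sound.
; A CloseDoor event lowers it by the same offset, reusing the open sound.
; The sound is played at the mesh's relative location rather than its world location.
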(event Custom|CloseDoor
  (bind _staticmesh (Variables|Default|GetStaticMesh))
  (bind _relativelocation (Variables|/Script/Engine.SceneComponent|GetRelativeLocation _staticmesh))
  (bind _returnvalue (Game|GetCurrentLevelName true))
  (if (Utilities|Enum|Equal(Enum) _returnvalue "L_Menu_Map")
    (Audio|PlaySoundatLocation "/Game/Main/Assets/Objects/Truck/Sound/SW_TruckDoor_Open.SW_TruckDoor_Open" (Variables|/Script/Engine.SceneComponent|GetRelativeLocation _staticmesh) "0, 0, 0" 1.0 1.0 0.0 0 0 0 0)
    (Components|MoveComponentTo (Variables|Default|GetStaticMesh) (Math|Vector|MakeVector (.x _relativelocation) (.y _relativelocation) (- (.z _relativelocation) 1.7e+02)) "0, 0, 0" true true 2.5 false)))

(event EventBeginPlay
  (bind _staticmesh (Variables|Default|GetStaticMesh))
  (bind _relativelocation (Variables|/Script/Engine.SceneComponent|GetRelativeLocation _staticmesh))
  (bind _returnvalue (Game|GetCurrentLevelName true))
  (if (Utilities|Enum|Equal(Enum) _returnvalue "L_Menu_Map")
    (Audio|PlaySoundatLocation "/Game/Main/Assets/Objects/Truck/Sound/SW_TruckDoor_Open.SW_TruckDoor_Open" (Variables|/Script/Engine.SceneComponent|GetRelativeLocation _staticmesh) "0, 0, 0" 1.0 1.0 0.0 0 0 0 0)
    (Components|MoveComponentTo (Variables|Default|GetStaticMesh) (Math|Vector|MakeVector (.x _relativelocation) (.y _relativelocation) (+ (.z _relativelocation) 1.7e+02)) "0, 0, 0" true true 2.5 false)))

(fn ConstructionScript)