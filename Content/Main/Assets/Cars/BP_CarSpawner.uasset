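; BP_CarSpawner keeps car traffic moving between a start point and an end point, one car at a time.
; On Tick, when no car is present, it waits a short random delay, spawns an AI-driven BP_Car at StartingPoint and sends it to EndPoint with AIMoveTo.
; On arrival it destroys the car and, after another random delay, clears IsCarPresent; a failed move leaves the flag set.
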(event EventTick
  (params (DeltaSeconds :type Float%20%28single-precision%29))
  (bind _startingpoint (Variables|Default|GetStartingPoint))
  (bind _rootcomponent (Variables|/Script/Engine.Actor|GetRootComponent _startingpoint))
  (if (not (Variables|Default|GetIsCarPresent))
    (Utilities|FlowControl|Delay (Math|Random|RandomFloatinRange 0.0 5.0))
    (Variables|Default|SetIsCarPresent true)
    (bind _returnvalue (AI|SpawnAIFromClass "/Game/Main/Assets/Cars/BP_Car.BP_Car_C" 0 (Transformation|GetWorldLocation _rootcomponent) (Transformation|GetWorldRotation _rootcomponent) false 0))
    (AI|AIMoveTo _returnvalue (Transformation|GetWorldLocation (Variables|/Script/Engine.Actor|GetRootComponent (Variables|Default|GetEndPoint))) 0 5.0 false
      (:OnSuccess
        (Actor|DestroyActor _returnvalue)
        (Utilities|FlowControl|Delay (Math|Random|RandomFloatinRange 0.0 5.0))
        (Variables|Default|SetIsCarPresent false)))))

(fn ConstructionScript)