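; BP_Car is a car NPC that varies its appearance and emits sound from its position.
; On BeginPlay a random MultiGate sets the static mesh to one of seven car models.
; Every Tick it plays a random entry from the Sounds array at the capsule's location at low volume, with no throttling between plays.
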(event EventBeginPlay
  ;[0.8128 1 0.7054] Randomize the NPC
  (Utilities|FlowControl|MultiGate true false -1
    (:Out%200
      (Components|StaticMesh|SetStaticMesh (Variables|Default|GetStaticMesh) "/Game/Main/Assets/Cars/SM_Car_1.SM_Car_1"))
    (:Out%201
      (Components|StaticMesh|SetStaticMesh (Variables|Default|GetStaticMesh) "/Game/Main/Assets/Cars/SM_Car_2.SM_Car_2"))
    (:Out%202
      (Components|StaticMesh|SetStaticMesh (Variables|Default|GetStaticMesh) "/Game/Main/Assets/Cars/SM_Car_3.SM_Car_3"))
    (:Out%203
      (Components|StaticMesh|SetStaticMesh (Variables|Default|GetStaticMesh) "/Game/Main/Assets/Cars/SM_Car_4.SM_Car_4"))
    (:Out%204
      (Components|StaticMesh|SetStaticMesh (Variables|Default|GetStaticMesh) "/Game/Main/Assets/Cars/SM_Car_5.SM_Car_5"))
    (:Out%205
      (Components|StaticMesh|SetStaticMesh (Variables|Default|GetStaticMesh) "/Game/Main/Assets/Cars/SM_Car_6.SM_Car_6"))
    (:Out%206
      (Components|StaticMesh|SetStaticMesh (Variables|Default|GetStaticMesh) "/Game/Main/Assets/Cars/SM_Car_7.SM_Car_7"))))

(event EventTick
  (params (DeltaSeconds :type Float%20%28single-precision%29))
  (Audio|PlaySoundatLocation (.OutItem (Utilities|Array|Random (Variables|Default|GetSounds))) (Transformation|GetWorldLocation (Variables|Collision|GetCapsuleComponent self)) "0, 0, 0" 0.05 1.0 0.0 0 0 0 0))

(fn ConstructionScript)