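; BP_NPCSpawner spawns customer NPCs one at a time and sends them to stand spots around the food truck.
; On BeginPlay it gathers the spot actors, picks a random unoccupied one, waits, then spawns an NPC at a random tagged TargetPoint.
; AIMoveTo walks it over; on arrival it faces the look target, claims the spot, animates and triggers the next spawn.
; The chain halts when no spot is free or a move fails.
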(event Custom|HandleNPCSpawn
  (bind _spottooccupy (Variables|Default|GetSpotToOccupy))
  ;[0.7699 1 0.9801] Spawn the random NPC
  (bind _outactors (Actor|GetAllActorsOfClasswithTag "/Script/Engine.TargetPoint" "NpcSpawn"))
  (bind _returnvalue (AI|SpawnAIFromClass "/Game/Main/Assets/NPCs/BP_NPC.BP_NPC_C" 0 (Transformation|GetWorldLocation (Variables|/Script/Engine.Actor|GetRootComponent (.OutItem (Utilities|Array|Random _outactors)))) "0, 0, 0" false 0))
  (Variables|Default|SetNPC _returnvalue)
  ;[0.8328 1 0.832] Make NPC walk to random unoccupied spot next to food truck
  (AI|AIMoveTo (Variables|Default|GetNPC) (Transformation|GetWorldLocation (Variables|/Script/Engine.Actor|GetRootComponent (Variables|Default|GetSpotToOccupy))) 0 5.0 false
    (:OnSuccess
      ;[1 1 1] Rotate NPC to face the food truck
      (bind _outactors_2 (Actor|GetAllActorswithTag "NpcLookTarget"))
      (Transformation|SetWorldRotation (Variables|/Script/Engine.Actor|GetRootComponent (Variables|Default|GetNPC)) (Math|Rotator|FindLookatRotation (Transformation|GetWorldLocation (Variables|/Script/Engine.Actor|GetRootComponent (Variables|Default|GetNPC))) (Transformation|GetActorLocation (Utilities|Array|Get(acopy) _outactors_2))) false false)
      ;[1 1 1] NPC arrived
      (Variables|/Game/Main/Assets/NPCs/NpcSpots/BP_NPCFoodTruckLocation.BP_NPCFoodTruckLocation_C|SetIsOccupied _spottooccupy true)
      (bind _asbp_npc (Utilities|Casting|CastToBP_NPC (Variables|Default|GetNPC)))
      (Variables|/Game/Main/Assets/NPCs/BP_NPC.BP_NPC_C|SetSpot _asbp_npc _spottooccupy)
      (Default|PlayArrivedAnimation _asbp_npc)
      (CallFunction|SpawnNewNPC))))

(event Custom|SpawnNewNPC
  ;[1 1 1] get random unoccupied food truck spot
  (bind _newparam (CallFunction|GetUnoccupiedFoodTruckSpots))
  (if (> (Utilities|Array|Length _newparam) 0)
    (Variables|Default|SetSpotToOccupy (.OutItem (Utilities|Array|Random _newparam)))
    (Utilities|FlowControl|Delay 1e+01)
    (CallFunction|HandleNPCSpawn)))

(event EventBeginPlay
  (bind _outactors (Actor|GetAllActorsOfClass "/Game/Main/Assets/NPCs/NpcSpots/BP_NPCFoodTruckLocation.BP_NPCFoodTruckLocation_C"))
  (Variables|Default|SetAllNPCStandSpots _outactors)
  (CallFunction|SpawnNewNPC))

(fn ConstructionScript)

(fn GetUnoccupiedFoodTruckSpots
  (for _array_element (Variables|Default|GetAllNPCStandSpots)
    (if (not (Variables|/Game/Main/Assets/NPCs/NpcSpots/BP_NPCFoodTruckLocation.BP_NPCFoodTruckLocation_C|GetIsOccupied _array_element))
      (Utilities|Array|Add (LocalVariables|GetUnoccupiedNPCStandSpots) _array_element)))
  (return (LocalVariables|GetUnoccupiedNPCStandSpots)))