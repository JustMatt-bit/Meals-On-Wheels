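; Customer NPC that arrives at a spot, places an order and leaves once it receives food.
; BeginPlay picks a random character mesh and matching gender flag.
; On arrival it waves, shows a widget, plays a gendered voice sound and starts the Spot's order, followed by random talk and idle montages.
; Receiving food triggers a random celebration, then it walks to a random NpcSpawn target point and destroys itself.
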(event Custom|PlayArrivedAnimation
  (bind _mesh (Variables|Character|GetMesh))
  (bind _returnvalue (Transformation|GetWorldLocation _mesh))
  ;[1 1 1] Wave
  (Animation|Montage|PlayMontage (Variables|Character|GetMesh) "/Game/Main/Assets/NPCs/Male/Adventurer/Animations/Standing-Greeting_Montage.Standing-Greeting_Montage"
    (:OnBlendOut
      (Development|SetHiddeninGame (Variables|Default|GetWidget1) false false)
      (if (Variables|Default|GetGenderMale)
        (Audio|PlaySoundatLocation (.OutItem (Utilities|Array|Random (Variables|Default|GetSoundsMale))) _returnvalue "0, 0, 0" 1.0 1.0 0.0 0 0 0 0)
        (else
          (Audio|PlaySoundatLocation (.OutItem (Utilities|Array|Random (Variables|Default|GetSoundsFemale))) _returnvalue "0, 0, 0" 1.0 1.0 0.0 0 0 0 0)))
      ;[1 1 1] Talk
      (Default|InitiateOrder (Variables|Default|GetSpot) self)
      (Utilities|FlowControl|MultiGate true false -1
        (:Out%200
          (Animation|Montage|PlayMontage (Variables|Character|GetMesh) "/Game/Main/Assets/NPCs/Male/Adventurer/Animations/Talk/Talking__1__Montage.Talking__1__Montage"
            (:OnBlendOut
              _)))
        (:Out%201
          (Animation|Montage|PlayMontage (Variables|Character|GetMesh) "/Game/Main/Assets/NPCs/Male/Adventurer/Animations/Talk/Talking_Montage.Talking_Montage"
            (:OnBlendOut
              _))))
      ;[1 1 1] Random Idle
      (Utilities|FlowControl|MultiGate true true -1
        (:Out%200
          (Animation|Montage|PlayMontage (Variables|Character|GetMesh) "/Game/Main/Assets/NPCs/Male/Adventurer/Animations/Idle/Breathing_Idle_Montage.Breathing_Idle_Montage"
            (:OnBlendOut
              _)))
        (:Out%201
          (Animation|Montage|PlayMontage (Variables|Character|GetMesh) "/Game/Main/Assets/NPCs/Male/Adventurer/Animations/Idle/Idle_Montage.Idle_Montage"
            (:OnBlendOut
              _)))
        (:Out%202
          (Animation|Montage|PlayMontage (Variables|Character|GetMesh) "/Game/Main/Assets/NPCs/Male/Adventurer/Animations/Idle/Idle__1__Montage.Idle__1__Montage"
            (:OnBlendOut
              _))))
      (Utilities|FlowControl|Delay 0.0))))

(event Custom|ReceivedFood
  ;[1 1 1] Show happiness
  (Utilities|FlowControl|MultiGate true false -1
    (:Out%200
      (Animation|Montage|PlayMontage (Variables|Character|GetMesh) "/Game/Main/Assets/NPCs/Male/Adventurer/Animations/Happy/Fist_Pump_Montage.Fist_Pump_Montage"
        (:OnBlendOut
          _)))
    (:Out%201
      (Animation|Montage|PlayMontage (Variables|Character|GetMesh) "/Game/Main/Assets/NPCs/Male/Adventurer/Animations/Happy/Clapping_Montage.Clapping_Montage"
        (:OnBlendOut
          _))))
  ;[1 1 1] Leave
  (bind _outactors (Actor|GetAllActorsOfClasswithTag "/Script/Engine.TargetPoint" "NpcSpawn"))
  (AI|AIMoveTo self (Transformation|GetWorldLocation (Variables|/Script/Engine.Actor|GetRootComponent (.OutItem (Utilities|Array|Random _outactors)))) 0 5.0 false
    (:OnSuccess
      (Actor|DestroyActor self))))

(event EventBeginPlay
  ;[0.8128 1 0.7054] Randomize the NPC
  (Utilities|FlowControl|MultiGate true false -1
    (:Out%200
      (Components|SkeletalMesh|SetSkeletalMeshAsset (Variables|Character|GetMesh) "/Game/Main/Assets/NPCs/Male/Adventurer/SM_Adventurer.SM_Adventurer")
      (Variables|Default|SetGenderMale true))
    (:Out%201
      (Components|SkeletalMesh|SetSkeletalMeshAsset (Variables|Character|GetMesh) "/Game/Main/Assets/NPCs/Male/Beach/Beach.Beach")
      (Variables|Default|SetGenderMale true))
    (:Out%202
      (Components|SkeletalMesh|SetSkeletalMeshAsset (Variables|Character|GetMesh) "/Game/Main/Assets/NPCs/Male/Suit/Suit__2_.Suit__2_")
      (Variables|Default|SetGenderMale true))
    (:Out%203
      (Components|SkeletalMesh|SetSkeletalMeshAsset (Variables|Character|GetMesh) "/Game/Main/Assets/NPCs/Male/Worker/Worker__1_.Worker__1_")
      (Variables|Default|SetGenderMale true))
    (:Out%204
      (Components|SkeletalMesh|SetSkeletalMeshAsset (Variables|Character|GetMesh) "/Game/Main/Assets/NPCs/Female/Formal/Formal__1_.Formal__1_")
      (Variables|Default|SetGenderMale false))
    (:Out%205
      (Components|SkeletalMesh|SetSkeletalMeshAsset (Variables|Character|GetMesh) "/Game/Main/Assets/NPCs/Female/Punk/Punk__3_.Punk__3_")
      (Variables|Default|SetGenderMale false))
    (:Out%206
      (Components|SkeletalMesh|SetSkeletalMeshAsset (Variables|Character|GetMesh) "/Game/Main/Assets/NPCs/Male/Casual/Casual.Casual")
      (Variables|Default|SetGenderMale true))
    (:Out%207
      (Components|SkeletalMesh|SetSkeletalMeshAsset (Variables|Character|GetMesh) "/Game/Main/Assets/NPCs/Female/Worker/Worker__2_.Worker__2_")
      (Variables|Default|SetGenderMale false))
    (:Out%208
      (Components|SkeletalMesh|SetSkeletalMeshAsset (Variables|Character|GetMesh) "/Game/Main/Assets/NPCs/Female/Suit/Suit__3_.Suit__3_")
      (Variables|Default|SetGenderMale false)))
  ;[1 1 1] Spawn the NPC behind buildings
  (Transformation|SetRelativeTransform (Variables|Character|GetMesh) (Math|Transform|MakeTransform "0.000000,0.000000,-90.000000" "0.000000,-90.000000,0.000000") false false))

(event Collision|EventActorBeginOverlap
  (params (OtherActor :type Actor%20Object%20Reference)))

(fn ConstructionScript)