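; Order station actor that takes an NPC's food order and pays out money when the matching food is delivered.
; NewOrder stores the NPC, spawns a ticket and sets the accepted class and payout, with only one food type (pizza) handled.
; A filled pizza box overlapping ItemCollision is destroyed with effects and sound.
; After a short delay, money spawns at the Arrow, the ticket is removed and the NPC is notified.
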(event OnComponentBeginOverlap(ItemCollision)
  (params (OverlappedComponent :type Primitive%20Component%20Object%20Reference) (OtherActor :type Actor%20Object%20Reference) (OtherComp :type Primitive%20Component%20Object%20Reference) (OtherBodyIndex :type Integer) (bFromSweep :type Boolean) (SweepResult :type Hit%20Result%20Structure%20%28by%20ref%29))
  (if (Utilities|ClassIsChildOf (Utilities|GetClass OtherActor) (Variables|Default|GetAcceptedBlueprint))
    (bind _asbp_pizzabox (Utilities|Casting|CastToBP_Pizzabox OtherActor))
    (if (Variables|/Game/Main/Assets/Objects/Pizzabox/BP_Pizzabox.BP_Pizzabox_C|GetHasPizza _asbp_pizzabox)
      (Niagara|SpawnSystematLocation "/Game/Main/Assets/Particles/NS_Confetti.NS_Confetti" (Transformation|GetWorldLocation (Variables|/Game/Main/Assets/Objects/Pizzabox/BP_Pizzabox.BP_Pizzabox_C|GetSM_Pizzabox_Bottom _asbp_pizzabox)))
      (Niagara|SpawnSystematLocation "/Game/Main/Assets/Particles/NS_Burst.NS_Burst" (Transformation|GetWorldLocation (Variables|/Game/Main/Assets/Objects/Pizzabox/BP_Pizzabox.BP_Pizzabox_C|GetSM_Pizzabox_Bottom _asbp_pizzabox)))
      (Actor|DestroyActor OtherActor)
      (Audio|PlaySound2D "/Game/Main/Assets/Blueprints/Orders/Audio/SW_Order_Success.SW_Order_Success" 1.0 1.0 0.0 0 0)
      (Utilities|FlowControl|Delay 1.0)
      (bind _returnvalue (Game|SpawnActorfromClass "/Game/Main/Assets/Objects/CashRegister/Money/BP_Money.BP_Money_C" (Transformation|GetWorldTransform (Variables|Default|GetArrow)) "Undefined" "MultiplyWithRoot" 0 0))
      (Variables|/Game/Main/Assets/Objects/CashRegister/Money/BP_Money.BP_Money_C|SetValue _returnvalue (Variables|Default|GetMoneyValue))
      (Actor|DestroyActor (Variables|Default|GetCurrentTicket))
      (Default|ReceivedFood (Variables|Default|GetCurrentNPC)))))

(event EventBeginPlay)

(event Collision|EventActorBeginOverlap
  (params (OtherActor :type Actor%20Object%20Reference)))

(event EventTick
  (params (DeltaSeconds :type Float%20%28single-precision%29)))

(fn ConstructionScript)

(fn NewOrder
  (params (NPC :type BP%20NPC%20Object%20Reference) (FoodType :type E_FoodTypes%20Enum :default "NewEnumerator0"))
  (Variables|Default|SetCurrentNPC NPC)
  (if (Utilities|Enum|Equal(Enum) FoodType "NewEnumerator0")
    (bind _returnvalue (Game|SpawnActorfromClass "/Game/Main/Assets/Blueprints/Orders/Pizza/BP_Ticket_Pizza.BP_Ticket_Pizza_C" (Transformation|GetWorldTransform (Variables|Default|GetArrow)) "Undefined" "MultiplyWithRoot" 0 0))
    (Variables|Default|SetCurrentTicket _returnvalue)
    (Variables|Default|SetAcceptedBlueprint "/Game/Main/Assets/Objects/Pizzabox/BP_Pizzabox.BP_Pizzabox_C")
    (Variables|Default|SetMoneyValue 15.0)))